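; Schar is a cover soldier that randomly pops up to aim and shows a key prompt while exposed.
; BeginPlay matches the capsule's Y position to one of four spots, setting that spot's flag and Q, W, E or R text.
; Tick uses Delays and a random roll to alternate cover and standing animations, toggling the prompt.
; It destroys the actor once Dead is set, which nothing here does.
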(event EventTick
  (params (DeltaSeconds :type Float%20%28single-precision%29))
  (if (Variables|Default|Getdead?)
    (Actor|DestroyActor))
  (if (Variables|Default|Getstanding?)
    (Rendering|SetVisibility (Variables|Default|GetKey) true false)
    (Components|Animation|PlayAnimation (Variables|Character|GetMesh) "/Game/Iheanacho/Assets/Characters/Soldier/Animations/AS_Soldier_CoverAim_Loop.AS_Soldier_CoverAim_Loop" false)
    (Utilities|FlowControl|Delay 2.0)
    (Rendering|SetVisibility (Variables|Default|GetKey) false false)
    (Components|Animation|PlayAnimation (Variables|Character|GetMesh) "/Game/Iheanacho/Assets/Characters/Soldier/Animations/AS_Soldier_CoverAim_StartReverse.AS_Soldier_CoverAim_StartReverse" false)
    (Components|Animation|PlayAnimation (Variables|Character|GetMesh) "/Game/Iheanacho/Assets/Characters/Soldier/Animations/AS_Soldier_CoverIdle.AS_Soldier_CoverIdle" false)
    (Utilities|FlowControl|Delay 1.0)
    (Variables|Default|Setstanding? false)
    (else
      (Rendering|SetVisibility (Variables|Default|GetKey) false false)
      (Utilities|FlowControl|Delay 2.0)
      (bind _output_get (Variables|Default|Setdenotion (Math|Random|RandomInteger 6)))
      (if (== _output_get 1)
        (Components|Animation|PlayAnimation (Variables|Character|GetMesh) "/Game/Iheanacho/Assets/Characters/Soldier/Animations/AS_Soldier_CoverAim_Start.AS_Soldier_CoverAim_Start" false)
        (Utilities|FlowControl|Delay 0.5)
        (Variables|Default|Setstanding? true)))))

(event Collision|EventActorBeginOverlap
  (params (OtherActor :type Actor%20Object%20Reference)))

(event EventBeginPlay
  (bind _key (Variables|Default|GetKey))
  (Rendering|SetVisibility (Variables|Default|GetKey) false false)
  (if (== (Math|Float|Truncate (.Y (Math|Vector|BreakVector (Transformation|GetWorldLocation (Variables|Collision|GetCapsuleComponent))))) -1500)
    (Rendering|Components|TextRender|SetText _key (Variables|Default|Getq1))
    (Variables|Default|Setset? true)
    (Variables|Default|Setspot1 true)
    (elif (== (Math|Float|Truncate (.Y (Math|Vector|BreakVector (Transformation|GetWorldLocation (Variables|Collision|GetCapsuleComponent))))) -1300)
      (Rendering|Components|TextRender|SetText _key (Variables|Default|Getw1))
      (Variables|Default|Setset? true)
      (Variables|Default|Setspot2 true)
      (elif (== (Math|Float|Truncate (.Y (Math|Vector|BreakVector (Transformation|GetWorldLocation (Variables|Collision|GetCapsuleComponent))))) -1100)
        (Rendering|Components|TextRender|SetText _key (Variables|Default|Gete1))
        (Variables|Default|Setset? true)
        (Variables|Default|Setspot3 true)
        (elif (== (Math|Float|Truncate (.Y (Math|Vector|BreakVector (Transformation|GetWorldLocation (Variables|Collision|GetCapsuleComponent))))) -900)
          (Rendering|Components|TextRender|SetText _key (Variables|Default|Getr1))
          (Variables|Default|Setset? true)
          (Variables|Default|Setspot4 true))))))

(fn ConstructionScript)